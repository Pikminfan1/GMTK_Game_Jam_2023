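; Player controller for mouse-driven item placement, showing the cursor and adding the placement Enhanced Input context.
; The slot 1 input cycles through the item list, spawning a replacement held item, while the clear input destroys it.
; Each tick, a cursor line trace moves the held item to the hit X/Y at zero height.
; Select input places it if BPI_ItemPlacement reports it spawnable, then spawns another of that class for repeat placement.
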(event `self.ReceiveBeginPlay`
  (bind _returnvalue (pcsubsystem `EnhancedInputLocalPlayerSubsystem` self))
  (set `self.bShowMouseCursor` true)
  (`/Engine/EditorBlueprintResources/StandardMacros.IsValid` _returnvalue
    (:`Is Valid`
      (`EnhancedInputSubsystemInterface.AddMappingContext` _returnvalue "/Game/_Game/Blueprints/ItemPlacementBlueprints/PlayerBlueprints/Input/IMC_PlaceItems.IMC_PlaceItems" 0 (struct)))))

(event `EnhancedInput|/Game/_Game/Blueprints/ItemPlacementBlueprints/PlayerBlueprints/Input/IA_ClearEquipSlot`
  (params (ActionValue :type Boolean) (ElapsedSeconds :type "Float (double-precision)") (TriggeredSeconds :type "Float (double-precision)") (InputAction :type "InputAction Object Reference" :default "/Game/_Game/Blueprints/ItemPlacementBlueprints/PlayerBlueprints/Input/IA_ClearEquipSlot.IA_ClearEquipSlot"))
  (bind _current_spawned_actor (`self.Current Spawned Actor`))
  (:`Started`
    (`/Engine/EditorBlueprintResources/StandardMacros.IsValid` (`self.Current Spawned Actor`)
      (:`Is Valid`
        (`self.K2_DestroyActor` _current_spawned_actor)
        (`self.SetIsEquipped` _current_spawned_actor)))))

(event `self.ReceiveTick`
  (params (DeltaSeconds :type "Float (single-precision)"))
  (`self.SetIsEquipped` (`self.Current Spawned Actor`))
  (if (`self.isEquipped?`)
    (`self.SetSelectedItemAndHoverAtMouseLocation` (`self.Current Spawned Actor`))))

(event `EnhancedInput|/Game/_Game/Blueprints/ItemPlacementBlueprints/PlayerBlueprints/Input/IA_EquipItemToSlot1`
  (params (ActionValue :type Boolean) (ElapsedSeconds :type "Float (double-precision)") (TriggeredSeconds :type "Float (double-precision)") (InputAction :type "InputAction Object Reference" :default "/Game/_Game/Blueprints/ItemPlacementBlueprints/PlayerBlueprints/Input/IA_EquipItemToSlot1.IA_EquipItemToSlot1"))
  (:`Started`
    (if (`self.isEquipped?`)
      (`self.K2_DestroyActor` (`self.Current Spawned Actor`))
      (`self.Equip Selected Item`)
      (else
        (`self.Equip Selected Item`)))))

(event `SetSelectedItemAndHoverAtMouseLocation`
  (params (SelectedItem :type "Actor Object Reference"))
  (`self.Get And Set Mouse X and Y Locations`)
  (`self.AttachSelectedItemAtCursorLocation` SelectedItem))

(event `Equip Selected Item`
  (bind _currentspawnedactor (`self.SpawnSelectedItem`))
  (bind _output_get (set `self.Current Spawned Actor` _currentspawnedactor))
  (`self.SetIsEquipped` _output_get))

(event `EnhancedInput|/Game/_Game/Blueprints/ItemPlacementBlueprints/PlayerBlueprints/Input/IA_SelectOrSpawnItem`
  (params (ActionValue :type Boolean) (ElapsedSeconds :type "Float (double-precision)") (TriggeredSeconds :type "Float (double-precision)") (InputAction :type "InputAction Object Reference" :default "/Game/_Game/Blueprints/ItemPlacementBlueprints/PlayerBlueprints/Input/IA_SelectOrSpawnItem.IA_SelectOrSpawnItem"))
  (:`Started`
    (if (`self.isEquipped?`)
      (bind _asbpi_item_placement (cast `/Game/_Game/Blueprints/ItemPlacementBlueprints/NewItemLogic/BPI_ItemPlacement` (`self.Current Spawned Actor`)))
      (bind _spawnable_ (`/Game/_Game/Blueprints/ItemPlacementBlueprints/NewItemLogic/BPI_ItemPlacement.GetItemSpawnable` _asbpi_item_placement))
      (if _spawnable_
        (`/Game/_Game/Blueprints/ItemPlacementBlueprints/NewItemLogic/BPI_ItemPlacement.SetItemPlaced` _asbpi_item_placement true)
        (set `self.Last Equipped Item` (`self.Current Spawned Actor`))
        (set `self.Current Spawned Actor` null)
        (bind _newequippeditem (`self.SpawnLastEquippedItem` (`self.Last Equipped Item`)))
        (set `self.Current Spawned Actor` _newequippeditem)))))

(fn `AttachSelectedItemAtCursorLocation`
  (params (SpawnedActor :type "Actor Object Reference"))
  (`self.K2_SetActorLocation` SpawnedActor (`self.MakeCursorLocation`) false false))

(fn `Get And Set Mouse X and Y Locations`
  (bind (_worldlocation _worlddirection) (`self.DeprojectMousePositionToWorld`))
  (bind _outhit (`KismetSystemLibrary.LineTraceSingle` :`Start` _worldlocation :`End` (+ _worldlocation (* _worlddirection (`self.RayLength`))) :`TraceChannel` "TraceTypeQuery1" :`DrawDebugType` "ForOneFrame" :`DrawTime` 0.0))
  (set `self.MouseX` (.x (`.Location` (`GameplayStatics.BreakHitResult` _outhit))))
  (set `self.MouseY` (.y (`.Location` (`GameplayStatics.BreakHitResult` _outhit)))))

(fn `MakeCursorLocation`
  (returns (CursorLocation :type "Vector Structure"))
  (return (`KismetMathLibrary.MakeVector` (`self.MouseX`) (`self.MouseY`))))

(fn `SetEditingMode`
  (if (not (`self.isEquipped?`))
    (set `self.EditingMode` true)
    (else
      (set `self.EditingMode` false)))
  (return))

(fn `SetIsEquipped`
  (params (EquippedActor :type "Actor Object Reference"))
  (if (`KismetSystemLibrary.IsValid` EquippedActor)
    (set `self.isEquipped?` true)
    (else
      (set `self.isEquipped?` false)))
  (return))

(fn `SpawnLastEquippedItem`
  (params (LastEquippedItem :type "Actor Object Reference"))
  (returns (NewEquippedItem :type "Actor Object Reference"))
  (bind _returnvalue (`|SpawnActorFromClass` (`GameplayStatics.GetObjectClass` LastEquippedItem) (`KismetMathLibrary.MakeTransform` (`self.MakeCursorLocation`)) "AlwaysSpawn" "MultiplyWithRoot" null null))
  (return _returnvalue))

(fn `SpawnSelectedItem`
  (returns (CurrentSpawnedActor :type "Actor Object Reference"))
  (bind _returnvalue (`|SpawnActorFromClass` (`|GetArrayItem` (`self.SelectedItemList`) (`self.ItemListIndex`)) (`KismetMathLibrary.MakeTransform` (`KismetMathLibrary.MakeVector` (`self.MouseX`) (`self.MouseY`))) "AlwaysSpawn" "MultiplyWithRoot" null null))
  (if (>= (`self.ItemListIndex`) (- (`KismetArrayLibrary.Array_Length` (`self.SelectedItemList`)) 1))
    (set `self.ItemListIndex` 0)
    (else
      (`/Engine/EditorBlueprintResources/StandardMacros.IncrementInt` (`self.ItemListIndex`)
        (:`  `
          _))))
  (return _returnvalue))

(fn `UserConstructionScript`)