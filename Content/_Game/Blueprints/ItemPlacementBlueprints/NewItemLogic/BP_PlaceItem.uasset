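; BP_PlaceItem is a placeable item actor that tracks whether it is placed and whether it can spawn at its current position.
; Bounds min/max comparisons test whether the item sits fully inside an overlapping BP_SpawnZone.
; The overlap check flags collision from the first other interface-implementing BP_PlaceItem's placed state, leaving it unchanged without overlaps.
; Callers pass both results into SetItemSpawnable, which requires no collision and being within bounds.
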(event `/Game/_Game/Blueprints/ItemPlacementBlueprints/NewItemLogic/BPI_ItemPlacement.SetItemPlaced`
  (params (`Placed?` :type Boolean))
  (`self.SetIsPlaced` `Placed?`))

(event `/Game/_Game/Blueprints/ItemPlacementBlueprints/NewItemLogic/BPI_ItemPlacement.SetItemSpawnable`
  (params (`Colliding?` :type Boolean) (`InZone?` :type Boolean))
  (`self.SetIsSpawnable` `Colliding?` `InZone?`))

(fn `Debug`
  (`KismetSystemLibrary.PrintString` (`KismetStringLibrary.Conv_BoolToString` (`self.IsCollidingWithOtherObjects?`)) true true (struct :`G` 0.66 :`B` 1.0 :`A` 1.0) 0.0)
  (`KismetSystemLibrary.PrintString` (`KismetStringLibrary.Conv_BoolToString` (`self.IsInsideZone?`)) true true (struct :`G` 0.66 :`B` 1.0 :`A` 1.0) 0.0)
  (`KismetSystemLibrary.PrintString` (`KismetStringLibrary.Conv_BoolToString` (`self.isSpawnable?`)) true true (struct :`G` 0.66 :`B` 1.0 :`A` 1.0) 0.0))

(fn `GetCollidingWithAnyItem?`
  (returns (`Colliding?` :type Boolean))
  (return (`self.IsCollidingWithOtherObjects?`)))

(fn `GetIsCompletelyInsideBox?`
  (returns (`IsInsideZone?` :type Boolean))
  (locals (SpawnZoneRef :type "/Game/_Game/Blueprints/ItemPlacementBlueprints/NewItemLogic/BP_SpawnZone Object Reference") (ItemMaxBoundCorner :type "Vector Structure") (ItemMinBoundCorner :type "Vector Structure") (ZoneMaxBoundCorner :type "Vector Structure") (ZoneMinBoundCorner :type "Vector Structure"))
  (bind (_itemmaxboundcorner_x _itemmaxboundcorner_y _itemmaxboundcorner_z) (`KismetMathLibrary.BreakVector` (`local.ItemMaxBoundCorner`)))
  (bind (_zonemaxboundcorner_x _zonemaxboundcorner_y _zonemaxboundcorner_z) (`KismetMathLibrary.BreakVector` (`local.ZoneMaxBoundCorner`)))
  (bind (_itemminboundcorner_x _itemminboundcorner_y _itemminboundcorner_z) (`KismetMathLibrary.BreakVector` (`local.ItemMinBoundCorner`)))
  (bind (_zoneminboundcorner_x _zoneminboundcorner_y _zoneminboundcorner_z) (`KismetMathLibrary.BreakVector` (`local.ZoneMinBoundCorner`)))
  (bind (_origin _boxextent) (`KismetSystemLibrary.GetComponentBounds` (`self.Item`)))
  (for _array_element (`PrimitiveComponent.GetOverlappingActors` (`self.Item`) "/Game/_Game/Blueprints/ItemPlacementBlueprints/NewItemLogic/BP_SpawnZone.BP_SpawnZone_C")
    (bind _asbp_spawn_zone (cast `/Game/_Game/Blueprints/ItemPlacementBlueprints/NewItemLogic/BP_SpawnZone` _array_element)
      (:`then`
        (bind _output_get (set `local.SpawnZoneRef` _asbp_spawn_zone))
        (set `local.ItemMaxBoundCorner` (+ _origin _boxextent))
        (set `local.ItemMinBoundCorner` (- _origin _boxextent))
        (bind (_origin_2 _boxextent_2) (`KismetSystemLibrary.GetComponentBounds` (`/Game/_Game/Blueprints/ItemPlacementBlueprints/NewItemLogic/BP_SpawnZone.CollisionBox` _output_get)))
        (set `local.ZoneMaxBoundCorner` (+ _origin_2 _boxextent_2))
        (set `local.ZoneMinBoundCorner` (- _origin_2 _boxextent_2))
        (set `self.IsInsideZone?` (and (and (< _itemmaxboundcorner_x _zonemaxboundcorner_x) (< _itemmaxboundcorner_y _zonemaxboundcorner_y) (< _itemmaxboundcorner_z _zonemaxboundcorner_z)) (and (> _itemminboundcorner_x _zoneminboundcorner_x) (> _itemminboundcorner_y _zoneminboundcorner_y) (> _itemminboundcorner_z _zoneminboundcorner_z))))
        (return (`self.IsInsideZone?`)))
      (:`CastFailed`
        (`KismetSystemLibrary.PrintString` "Need to inherit zone better")))))

(fn `GetIsPlaced`
  (returns (`isPlaced?` :type Boolean))
  (return (`self.isPlaced?`)))

(fn `GetIsSpawnable`
  (returns (`isSpawnable?` :type Boolean))
  (return (`self.isSpawnable?`)))

(fn `GetItemPlaced`
  (returns (`Placed?` :type Boolean))
  (bind _isplaced_ (`self.GetIsPlaced`))
  (return _isplaced_))

(fn `GetItemSpawnable`
  (returns (`Spawnable?` :type Boolean))
  (bind _isspawnable_ (`self.GetIsSpawnable`))
  (return _isspawnable_))

(fn `IsCollidingWithPlacedObject?`
  (bind _overlappingactors (`PrimitiveComponent.GetOverlappingActors` (`self.Item`) "BP_PlaceItem_C"))
  (if (`KismetArrayLibrary.Array_IsNotEmpty` _overlappingactors)
    (for _array_element _overlappingactors
      (if (== _array_element self)
        (`self.SetIsCollidingWithObjects` false)
        (else
          (bind _asbpi_item_placement (cast `/Game/_Game/Blueprints/ItemPlacementBlueprints/NewItemLogic/BPI_ItemPlacement` _array_element)
            (:`then`
              (bind _placed_ (`/Game/_Game/Blueprints/ItemPlacementBlueprints/NewItemLogic/BPI_ItemPlacement.GetItemPlaced` _asbpi_item_placement))
              (if _placed_
                (`self.SetIsCollidingWithObjects` true)
                (else
                  (`self.SetIsCollidingWithObjects` false)))
              (return))
            (:`CastFailed`
              (`self.SetIsCollidingWithObjects` false))))))
    (return)))

(fn `SetIsCollidingWithObjects`
  (params (`isColliding?` :type Boolean))
  (set `self.IsCollidingWithOtherObjects?` `isColliding?`)
  (return))

(fn `SetIsPlaced`
  (params (Placed :type Boolean))
  (set `self.isPlaced?` Placed)
  (return))

(fn `SetIsSpawnable`
  (params (`isColliding?` :type Boolean) (isWithinBounds :type Boolean))
  (set `self.isSpawnable?` (and (not `isColliding?`) isWithinBounds)))

(fn `UserConstructionScript`)