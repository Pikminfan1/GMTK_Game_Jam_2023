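; Chest variant of a placeable item, which tracks whether it can be spawned at its current position.
; Each tick it runs a collision check against placed objects through BPI_ItemPlacement on itself.
; It then passes the colliding and completely-inside-box flags to SetItemSpawnable.
; The final spawnable branch is a debug leftover with its print disconnected.
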(event `self.ReceiveTick`
  (params (DeltaSeconds :type "Float (single-precision)"))
  (`parent.ReceiveTick` DeltaSeconds)
  (bind _asbpi_item_placement (cast `/Game/_Game/Blueprints/ItemPlacementBlueprints/NewItemLogic/BPI_ItemPlacement` self))
  (`self.IsCollidingWithPlacedObject?` _asbpi_item_placement)
  (bind _colliding_ (`self.GetCollidingWithAnyItem?`))
  (bind _isinsidezone_ (`self.GetIsCompletelyInsideBox?`))
  (`self.SetItemSpawnable` _asbpi_item_placement _colliding_ _isinsidezone_)
  ;[1 1 1] debug only object that is not placed, not colliding with other items and is within bounds will print true
  (bind _isspawnable_ (`self.GetIsSpawnable`))
  (if _isspawnable_
    _))

(fn `UserConstructionScript`
  (`parent.UserConstructionScript`))