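; Cursor controller that spawns a BP_Ball in the world at the point under the mouse on left click.
; It deprojects the mouse position from player 0's controller and runs a Visibility line trace along that direction for RayLength, with persistent debug drawing.
; The hit actor and location are logged, and the ball spawns at the hit location without checking whether the trace hit anything.
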(event `Key|LeftMouseButton`
  (params (Key :type "Key Structure"))
  (bind (_worldlocation _worlddirection) (`self.DeprojectMousePositionToWorld` (`GameplayStatics.GetPlayerController` 0)))
  (:`Pressed`
    (bind _outhit (`KismetSystemLibrary.LineTraceSingle` :`Start` _worldlocation :`End` (+ _worldlocation (* _worlddirection (`self.RayLength`))) :`TraceChannel` "TraceTypeQuery1" :`DrawDebugType` "Persistent"))
    (`KismetSystemLibrary.LogString` (`KismetSystemLibrary.GetDisplayName` (`.HitActor` (`GameplayStatics.BreakHitResult` _outhit))))
    (`KismetSystemLibrary.LogString` (`KismetStringLibrary.Conv_VectorToString` (`.Location` (`GameplayStatics.BreakHitResult` _outhit))))
    (`|SpawnActorFromClass` "/Game/_Game/Blueprints/BP_Ball.BP_Ball_C" (`KismetMathLibrary.Conv_VectorToTransform` (`.Location` (`GameplayStatics.BreakHitResult` _outhit))) "Undefined" "MultiplyWithRoot" null null)))

(fn `UserConstructionScript`)