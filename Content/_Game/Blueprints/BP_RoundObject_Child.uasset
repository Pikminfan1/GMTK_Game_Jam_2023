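; Round placeable object that checks every tick whether its current position is a valid spot for spawning.
; It counts as in bounds when the axis-aligned bounds of its Object component lie strictly inside an overlapping BP_PlacementZone's collision box.
; Collision depends on whether the first overlapping actor, ignoring itself and zones, is a BP_Object.
; Tick passes both results to the BP_PlayerMouse pawn as IsSpawnable and Colliding, with debug prints.
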(event `self.ReceiveBeginPlay`
  (`parent.ReceiveBeginPlay`)
  (bind _asbp_player_mouse (cast `/Game/_Game/Blueprints/BP_PlayerMouse` (`GameplayStatics.GetPlayerPawn` 0)))
  (set `self.MouseCharacter` _asbp_player_mouse))

(event `self.ReceiveTick`
  (params (DeltaSeconds :type "Float (single-precision)"))
  (bind _mousecharacter (`self.MouseCharacter`))
  (`parent.ReceiveTick` DeltaSeconds)
  (bind _iscompletelyinsidezone (`self.isCompletelyInsideBox?`))
  (bind _colliding_ (`self.isCollidingWithAnyMesh?`))
  (if _colliding_
    (set `/Game/_Game/Blueprints/BP_PlayerMouse.Colliding?` true _mousecharacter)
    (else
      (set `/Game/_Game/Blueprints/BP_PlayerMouse.Colliding?` false _mousecharacter)))
  (if _iscompletelyinsidezone
    (set `/Game/_Game/Blueprints/BP_PlayerMouse.isSpawnable?` true _mousecharacter)
    (else
      (set `/Game/_Game/Blueprints/BP_PlayerMouse.isSpawnable?` false _mousecharacter)))
  (`KismetSystemLibrary.PrintString` "IsColliding" (`self.isColliding?`) true (struct :`G` 0.66 :`B` 1.0 :`A` 1.0) 0.0)
  (`KismetSystemLibrary.PrintString` "isInBounds" (`self.isSpawnable?`) true (struct :`G` 0.66 :`B` 1.0 :`A` 1.0) 0.0))

(fn `isCollidingWithAnyMesh?`
  (returns (`Colliding?` :type Boolean))
  (bind _overlappingactors (`PrimitiveComponent.GetOverlappingActors` (`self.Object`) null))
  (`parent.isCollidingWithAnyMesh?`)
  (if (`KismetArrayLibrary.Array_IsNotEmpty` _overlappingactors)
    (for _array_element _overlappingactors
      (if (== _array_element self)
        (set `self.isColliding?` false)
        (else
          (bind _returnvalue (`GameplayStatics.GetObjectClass` _array_element))
          (if (not (`KismetMathLibrary.ClassIsChildOf` _returnvalue "/Game/_Game/Blueprints/BP_PlacementZone.BP_PlacementZone_C"))
            (if (`KismetMathLibrary.ClassIsChildOf` _returnvalue "/Game/_Game/Blueprints/BP_Object.BP_Object_C")
              (set `self.isColliding?` true)
              (else
                (set `self.isColliding?` false)))
            (return (`self.isColliding?`))))))
    (else
      (set `self.isColliding?` false)))
  (return (`self.isColliding?`)))

(fn `isCompletelyInsideBox?`
  (locals (ObjectMaxBoundCorner :type "Vector Structure") (ObjectMinBoundCorner :type "Vector Structure") (ZoneMaxBoundCorner :type "Vector Structure") (ZoneMinBoundCorner :type "Vector Structure"))
  (bind (_objectmaxboundcorner_x _objectmaxboundcorner_y _objectmaxboundcorner_z) (`KismetMathLibrary.BreakVector` (`local.ObjectMaxBoundCorner`)))
  (bind (_zonemaxboundcorner_x _zonemaxboundcorner_y _zonemaxboundcorner_z) (`KismetMathLibrary.BreakVector` (`local.ZoneMaxBoundCorner`)))
  (bind (_objectminboundcorner_x _objectminboundcorner_y _objectminboundcorner_z) (`KismetMathLibrary.BreakVector` (`local.ObjectMinBoundCorner`)))
  (bind (_zoneminboundcorner_x _zoneminboundcorner_y _zoneminboundcorner_z) (`KismetMathLibrary.BreakVector` (`local.ZoneMinBoundCorner`)))
  (bind (_origin _boxextent) (`KismetSystemLibrary.GetComponentBounds` (`self.Object`)))
  (`parent.isCompletelyInsideBox?`)
  (for _array_element (`PrimitiveComponent.GetOverlappingActors` (`self.Object`) "/Game/_Game/Blueprints/BP_PlacementZone.BP_PlacementZone_C")
    (bind _asbp_placement_zone (cast `/Game/_Game/Blueprints/BP_PlacementZone` _array_element))
    (set `local.ObjectMaxBoundCorner` (+ _origin _boxextent))
    (set `local.ObjectMinBoundCorner` (- _origin _boxextent))
    (bind (_origin_2 _boxextent_2) (`KismetSystemLibrary.GetComponentBounds` (`/Game/_Game/Blueprints/BP_PlacementZone.CollisionBox` _asbp_placement_zone)))
    (set `local.ZoneMaxBoundCorner` (+ _origin_2 _boxextent_2))
    (set `local.ZoneMinBoundCorner` (- _origin_2 _boxextent_2))
    (bind _output_get (set `self.isSpawnable?` (and (and (< _objectmaxboundcorner_x _zonemaxboundcorner_x) (< _objectmaxboundcorner_y _zonemaxboundcorner_y) (< _objectmaxboundcorner_z _zonemaxboundcorner_z)) (and (> _objectminboundcorner_x _zoneminboundcorner_x) (> _objectminboundcorner_y _zoneminboundcorner_y) (> _objectminboundcorner_z _zoneminboundcorner_z)))))
    (`KismetSystemLibrary.PrintString` "Hello" _output_get true (struct :`G` 0.66 :`B` 1.0 :`A` 1.0) 0.0)))

(fn `UserConstructionScript`
  (`parent.UserConstructionScript`))