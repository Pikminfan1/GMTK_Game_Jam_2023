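; BP_Object_Child is a placeable object that checks whether it sits entirely inside a BP_PlacementZone.
; Each Tick, after the parent Tick, it loops over overlapping zones and compares world-space min/max bound corners against each zone's CollisionBox on all three axes.
; The result sets IsSpawnable, gates a "Hello" debug print, and is followed by the parent check inside the loop, so nothing updates without an overlapping zone.
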(event `self.ReceiveTick`
  (params (DeltaSeconds :type "Float (single-precision)"))
  (`parent.ReceiveTick` DeltaSeconds)
  (`self.isCompletelyInsideBox?`))

(fn `isCompletelyInsideBox?`
  (locals (ObjectMaxBoundCorner :type "Vector Structure") (ObjectMinBoundCorner :type "Vector Structure") (ZoneMaxBoundCorner :type "Vector Structure") (ZoneMinBoundCorner :type "Vector Structure"))
  (bind (_objectmaxboundcorner_x _objectmaxboundcorner_y _objectmaxboundcorner_z) (`KismetMathLibrary.BreakVector` (`local.ObjectMaxBoundCorner`)))
  (bind (_zonemaxboundcorner_x _zonemaxboundcorner_y _zonemaxboundcorner_z) (`KismetMathLibrary.BreakVector` (`local.ZoneMaxBoundCorner`)))
  (bind (_objectminboundcorner_x _objectminboundcorner_y _objectminboundcorner_z) (`KismetMathLibrary.BreakVector` (`local.ObjectMinBoundCorner`)))
  (bind (_zoneminboundcorner_x _zoneminboundcorner_y _zoneminboundcorner_z) (`KismetMathLibrary.BreakVector` (`local.ZoneMinBoundCorner`)))
  (bind (_origin _boxextent) (`KismetSystemLibrary.GetComponentBounds` (`self.Object`)))
  (for _array_element (`PrimitiveComponent.GetOverlappingActors` (`self.Object`) "/Game/_Game/Blueprints/BP_PlacementZone.BP_PlacementZone_C")
    (bind _asbp_placement_zone (cast `/Game/_Game/Blueprints/BP_PlacementZone` _array_element))
    (set `local.ObjectMaxBoundCorner` (+ _origin _boxextent))
    (set `local.ObjectMinBoundCorner` (- _origin _boxextent))
    (bind (_origin_2 _boxextent_2) (`KismetSystemLibrary.GetComponentBounds` (`/Game/_Game/Blueprints/BP_PlacementZone.CollisionBox` _asbp_placement_zone)))
    (set `local.ZoneMaxBoundCorner` (+ _origin_2 _boxextent_2))
    (set `local.ZoneMinBoundCorner` (- _origin_2 _boxextent_2))
    (bind _output_get (set `self.isSpawnable?` (and (and (< _objectmaxboundcorner_x _zonemaxboundcorner_x) (< _objectmaxboundcorner_y _zonemaxboundcorner_y) (< _objectmaxboundcorner_z _zonemaxboundcorner_z)) (and (> _objectminboundcorner_x _zoneminboundcorner_x) (> _objectminboundcorner_y _zoneminboundcorner_y) (> _objectminboundcorner_z _zoneminboundcorner_z)))))
    (`KismetSystemLibrary.PrintString` "Hello" _output_get true (struct :`G` 0.66 :`B` 1.0 :`A` 1.0) 0.0)
    (`parent.isCompletelyInsideBox?`)))

(fn `UserConstructionScript`
  (`parent.UserConstructionScript`))